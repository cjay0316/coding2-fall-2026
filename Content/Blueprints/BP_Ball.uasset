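; BP_Ball is a ball item that can be picked up, used and dropped.
; Pickup turns off the sphere's collision and returns its ItemType.
; Drop restores collision, enables physics and launches the sphere along its forward vector with a mass-independent velocity impulse, so it behaves like a throw.
; Use only prints a "Bounce" message.
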(event `/Game/Blueprints/BPI_Item.Drop`
  (bind _sphere (`self.Sphere`))
  (`PrimitiveComponent.SetCollisionEnabled` _sphere "QueryAndPhysics")
  (`PrimitiveComponent.SetSimulatePhysics` _sphere true)
  (`PrimitiveComponent.AddImpulse` _sphere (* (`SceneComponent.GetForwardVector` _sphere) 1000.0) "None" true))

(event `/Game/Blueprints/BPI_Item.Use`
  (`KismetSystemLibrary.PrintText` "Bounce"))

(fn `Pickup`
  (params (Owner :type "/Game/Blueprints/BPC_Interact Object Reference (by ref)"))
  (returns (ItemType :type "/Game/Blueprints/E_Item Enum"))
  (`PrimitiveComponent.SetCollisionEnabled` (`self.Sphere`) "NoCollision")
  (return (`self.ItemType`)))

(fn `UserConstructionScript`)