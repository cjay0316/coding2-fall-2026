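; BP_HealthKit is a health kit item actor that can be picked up, dropped and used.
; Pickup disables collision on the Cube and returns the ItemType, while Drop restores collision and physics and launches the Cube forward with a velocity-change impulse.
; Use only prints a "Health restored!" message, plays a 2D sound and destroys the actor, without changing any health value.
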(event `/Game/Blueprints/BPI_Item.Drop`
  (bind _cube (`self.Cube`))
  (`PrimitiveComponent.SetCollisionEnabled` _cube "QueryAndPhysics")
  (`PrimitiveComponent.SetSimulatePhysics` _cube true)
  (`PrimitiveComponent.AddImpulse` _cube (* (`SceneComponent.GetForwardVector` _cube) 1000.0) "None" true))

(event `/Game/Blueprints/BPI_Item.Use`
  (`KismetSystemLibrary.PrintText` "Health restored!")
  (`GameplayStatics.PlaySound2D` "/Engine/VREditor/Sounds/VR_shep_scale_up_03.VR_shep_scale_up_03" 1.0 1.0 0.0 null null)
  (`self.K2_DestroyActor`))

(fn `Pickup`
  (params (Owner :type "/Game/Blueprints/BPC_Interact Object Reference (by ref)"))
  (returns (ItemType :type "/Game/Blueprints/E_Item Enum"))
  (`PrimitiveComponent.SetCollisionEnabled` (`self.Cube`) "NoCollision")
  (return (`self.ItemType`)))

(fn `UserConstructionScript`)