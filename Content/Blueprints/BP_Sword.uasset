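; BP_Sword is a sword item that can be picked up, dropped and used by the player.
; Pickup disables mesh collision and returns the item type, while Drop restores collision, enables physics and throws the mesh along its forward vector with a velocity-change impulse.
; Use checks HasSword, then passes a DoOnce with no reset wired to call PlayMontage on the player's mesh and print a placeholder swoosh message.
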(event `/Game/Blueprints/BPI_Item.Drop`
  (bind _staticmesh (`self.StaticMesh`))
  (`PrimitiveComponent.SetCollisionEnabled` _staticmesh "QueryAndPhysics")
  (`PrimitiveComponent.SetSimulatePhysics` _staticmesh true)
  (`PrimitiveComponent.AddImpulse` _staticmesh (* (`SceneComponent.GetForwardVector` _staticmesh) 1000.0) "None" true))

(event `/Game/Blueprints/BPI_Item.Use`
  (if (`self.Has Sword?`)
    (`/Engine/EditorBlueprintResources/StandardMacros.DoOnce` false
      (:`Completed`
        (`|PlayMontage` (`Character.Mesh` (`self.Player`))
          (:`then`
            (`KismetSystemLibrary.PrintText` "Swooosh")))))))

(fn `Pickup`
  (params (Owner :type "/Game/Blueprints/BPC_Interact Object Reference (by ref)"))
  (returns (ItemType :type "/Game/Blueprints/E_Item Enum"))
  (`PrimitiveComponent.SetCollisionEnabled` (`self.StaticMesh`) "NoCollision")
  (return (`self.ItemType`)))

(fn `UserConstructionScript`)