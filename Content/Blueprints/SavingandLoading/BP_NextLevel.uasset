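; BP_NextLevel is a level transition trigger that saves the player's state and opens a destination level.
; When BP_FirstPersonCharacter overlaps it, it passes the belt and backpack inventory component contents to GM_SaveLoad's Save.
; The saved last position comes from the actor's LoadingPOS world transform rather than the player's own.
; It then opens the Destination level by object reference.
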(event `self.ReceiveActorBeginOverlap`
  (params (OtherActor :type "Actor Object Reference"))
  (bind _asbp_first_person_character (cast `/Game/FirstPerson/Blueprints/BP_FirstPersonCharacter` OtherActor)) ; Was it the player who walked into the checkpoint?
  (bind _asgm_save_load (cast `/Game/Blueprints/SavingandLoading/GM_SaveLoad` (`GameplayStatics.GetGameMode`))) ; Get game mode
  (`/Game/Blueprints/SavingandLoading/GM_SaveLoad.Save` _asgm_save_load (`/Game/Blueprints/BPC_Inventory.E Invt` (`/Game/FirstPerson/Blueprints/BP_FirstPersonCharacter.BPC_InvBelt` _asbp_first_person_character)) (`/Game/Blueprints/BPC_Inventory.E Invt` (`/Game/FirstPerson/Blueprints/BP_FirstPersonCharacter.BPC_InvBackpack` _asbp_first_person_character)) (`SceneComponent.K2_GetComponentToWorld` (`self.Loading POS`))) ; Save the player value
  (`GameplayStatics.OpenLevelBySoftObjectPtr` (`self.Destination`)))

(fn `UserConstructionScript`)