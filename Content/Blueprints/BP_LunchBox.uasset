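; BP_LunchBox is a lunch box item that can be picked up, dropped and used.
; Pickup disables collision on its Cube component.
; Drop restores collision, enables physics simulation and launches the Cube along its own forward vector with a mass-independent impulse.
; Use only prints an eating message, with no other gameplay effect.
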(event `/Game/Blueprints/BPI_Item.Pickup`
  (params (Owner :type "/Game/Blueprints/BPC_Interact Object Reference (by ref)"))
  (`PrimitiveComponent.SetCollisionEnabled` (`self.Cube`) "NoCollision"))

(event `/Game/Blueprints/BPI_Item.Drop`
  (bind _cube (`self.Cube`))
  (`PrimitiveComponent.SetCollisionEnabled` _cube "QueryAndPhysics")
  (`PrimitiveComponent.SetSimulatePhysics` _cube true)
  (`PrimitiveComponent.AddImpulse` _cube (* (`SceneComponent.GetForwardVector` _cube) 1000.0) "None" true))

(event `/Game/Blueprints/BPI_Item.Use`
  (`KismetSystemLibrary.PrintText` "Yum yum"))

(fn `UserConstructionScript`)