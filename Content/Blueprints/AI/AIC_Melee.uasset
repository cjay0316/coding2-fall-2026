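; AI controller for a melee AI that turns perception of actors not tagged "AI" into StateTree events.
; Sight stores the target and sends an Attacking event, while hearing and damage store a point of interest and send an Investigating event.
; Losing sight starts a retriggerable delay, after which, if CanSeePlayer is false, the target's current location becomes the point of interest and the target is cleared.
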(event `self.AIPerception.OnTargetPerceptionUpdated`
  (params (Actor :type "Actor Object Reference") (Stimulus :type "AIStimulus Structure"))
  (bind (_age _expirationage _strength _stimuluslocation _receiverlocation _tag _bsuccessfullysensed) (break `AIStimulus` Stimulus))
  (if (not (`self.ActorHasTag` Actor "AI"))
    (bind _returnvalue (`AIPerceptionSystem.GetSenseClassForStimulus` Stimulus))
    (switch `string` (`KismetSystemLibrary.GetClassDisplayName` _returnvalue)
      (:`AISense_Sight`
        (`self.HandleSight` _bsuccessfullysensed Actor))
      (:`AISense_Hearing`
        (`self.HandleSound` _stimuluslocation))
      (:`AISense_Damage`
        (`self.HandleDamage` Actor _stimuluslocation)))))

(event `self.ReceivePossess`
  (params (PossessedPawn :type "Pawn Object Reference"))
  (set `self.Possessed Pawn` PossessedPawn))

(event `LoseSightDelay`
  (set `self.Can See Player` false)
  (`KismetSystemLibrary.RetriggerableDelay` (`self.Lose Sight Duration`))
  (if (not (`self.Can See Player`))
    (set `self.PointOfInterest` (`self.K2_GetActorLocation` (`self.Target Actor`)))
    (set `self.Target Actor` null)))

(fn `HandleDamage`
  (params (Attacker :type "Actor Object Reference") (PointOfInterest :type "Vector Structure"))
  (set `self.PointOfInterest` PointOfInterest)
  (`StateTreeComponent.SendStateTreeEvent` (`self.StateTreeAI`) (make `StateTreeEvent` :`Tag` (struct :`TagName` "AI.Event.Investigating"))))

(fn `HandleSight`
  (params (SuccessfullySensed :type Boolean) (TargetActor :type "Actor Object Reference"))
  (if SuccessfullySensed
    (set `self.Target Actor` TargetActor) ; Assign Target
    (`StateTreeComponent.SendStateTreeEvent` (`self.StateTreeAI`) (make `StateTreeEvent` :`Tag` (struct :`TagName` "AI.Event.Attacking")))
    (else
      (`self.LoseSightDelay`))))

(fn `HandleSound`
  (params (Location :type "Vector Structure"))
  (set `self.PointOfInterest` Location)
  (`StateTreeComponent.SendStateTreeEvent` (`self.StateTreeAI`) (make `StateTreeEvent` :`Tag` (struct :`TagName` "AI.Event.Investigating"))))

(fn `UserConstructionScript`)