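; Security camera Blueprint that spots the player and sends BP_DumDum guards to the target's location.
; HandleSight records visibility and moves a Looking camera to Investigating, which after a one-second delay escalates to Alert or returns to Looking.
; Alert re-calls itself every second, redirecting all guards while sight holds, then falls back to Investigating.
; Each state swaps the mesh material as a visual indicator.
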(event `HandleSight`
  (params (SuccessfullySensed :type Boolean) (Target :type "Actor Object Reference"))
  (set `self.CurentlySeesPlayer` SuccessfullySensed)
  (switch `/Game/Blueprints/AI/E_CamState` (`self.CameraState`)
    (:`NewEnumerator0`
      (`self.Invetigating` (`self.CurentlySeesPlayer`)))))

(event `Invetigating`
  (params (Sensed :type Boolean))
  (set `self.CameraState` "NewEnumerator1")
  (`PrimitiveComponent.SetMaterial` (`self.StaticMesh`) 0 "/Game/BlockingStarterPack/Materials/Blocking/TriPlanarLocalAligned/MI_DevYellow_TPLA.MI_DevYellow_TPLA") ; Chnage color to yellow
  (`KismetSystemLibrary.Delay` 1.0)
  (if (`self.CurentlySeesPlayer`)
    (`self.Alert`)
    (else
      (`self.Looking`))))

(event `Alert`
  (if (`self.CurentlySeesPlayer`)
    (set `self.CameraState` "NewEnumerator2")
    (`PrimitiveComponent.SetMaterial` (`self.StaticMesh`) 0 "/AnimationSharing/AnimSharingRed.AnimSharingRed")
    (bind _outactors (`GameplayStatics.GetAllActorsOfClass` "/Game/Blueprints/AI/BP_DumDum.BP_DumDum_C"))
    (for _array_element _outactors
      (`/Game/Blueprints/AI/BP_DumDum.GoToSecPoint` _array_element (`self.K2_GetActorLocation` (stale `HandleSight` Target))))
    (`KismetSystemLibrary.Delay` 1.0)
    (`self.Alert`)
    (else
      (`self.Invetigating` false))))

(event `Looking`
  (set `self.CameraState` "NewEnumerator0")
  (`PrimitiveComponent.SetMaterial` (`self.StaticMesh`) 0 "/Engine/EditorMaterials/MatineeCam_mat.MatineeCam_mat"))

(fn `UserConstructionScript`)