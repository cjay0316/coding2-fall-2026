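; AI controller that handles sight perception for a possessed BP_SecurityCamera pawn.
; On possession it caches the camera reference.
; Perception updates, except from actors tagged "None", are routed by stimulus sense class, with only sight handled.
; HandleSight prints a debug message on gain or loss of sight, then forwards the result and target to the camera if valid.
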(event `self.AIPerception.OnTargetPerceptionUpdated`
  (params (Actor :type "Actor Object Reference") (Stimulus :type "AIStimulus Structure"))
  (if (not (`self.ActorHasTag` Actor "None"))
    (bind _returnvalue (`AIPerceptionSystem.GetSenseClassForStimulus` Stimulus))
    (switch `string` (`KismetSystemLibrary.GetClassDisplayName` _returnvalue)
      (:`AISense_Sight`
        (`self.HandleSight` (`.bSuccessfullySensed` (break `AIStimulus` Stimulus)) Actor)))))

(event `self.ReceivePossess`
  (params (PossessedPawn :type "Pawn Object Reference"))
  (bind _asbp_security_camera (cast `/Game/Blueprints/AI/BP_SecurityCamera` PossessedPawn))
  (set `self.As BP Security Camera` _asbp_security_camera))

(fn `HandleSight`
  (params (SuccessfullySensed :type Boolean) (Target :type "Actor Object Reference"))
  (if SuccessfullySensed
    (`KismetSystemLibrary.PrintText` "I see the player now!")
    (else
      (`KismetSystemLibrary.PrintText` "I don't see the player now!" true true (struct :`R` 1.0 :`G` 0.0288 :`B` 0.008267 :`A` 1.0))))
  (bind _as_bp_security_camera (`self.As BP Security Camera`)
    (:`then`
      (`/Game/Blueprints/AI/BP_SecurityCamera.HandleSight` _as_bp_security_camera SuccessfullySensed Target))
    (:`else`)))

(fn `UserConstructionScript`)