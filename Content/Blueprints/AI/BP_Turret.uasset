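; BP_Turret is an AI turret that aims and fires BP_Bullet at a sensed target.
; HandleSight stores the target and starts Attack, or clears it when sensing fails.
; Attack spawns bullets at BulletSpawn, re-calling itself after a RoundsPerMinute / 60 second delay while the target is valid.
; Tick rotates Pivot toward the target's location plus a fraction of its velocity to lead shots.
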(event `/Game/Blueprints/AI/BPI_Percetor.HandleSight`
  (params (target :type "Actor Object Reference") (location :type "Vector Structure") (SuccessfullySensed :type Boolean))
  (if SuccessfullySensed
    (set `self.Enenmy Target` target)
    (`self.Attack`)
    (else
      (set `self.Enenmy Target` null))))

(event `Attack`
  (`self.Enenmy Target`
    (:`then`
      (`|SpawnActorFromClass` "/Game/Blueprints/AI/BP_Bullet.BP_Bullet_C" (`SceneComponent.K2_GetComponentToWorld` (`self.BulletSpawn`)) "Undefined" "MultiplyWithRoot" null self)
      (`KismetSystemLibrary.Delay` (/ (`self.RoundsPerMinute`) 60.0))
      (`self.Attack`))
    (:`else`)))

(event `self.ReceiveTick`
  (params (DeltaSeconds :type "Float (single-precision)"))
  (bind _enenmy_target (`self.Enenmy Target`))
  (`self.Enenmy Target`
    (:`then`
      (`SceneComponent.K2_SetWorldRotation` (`self.Pivot`) (`KismetMathLibrary.FindLookAtRotation` (`SceneComponent.K2_GetComponentLocation` (`self.DefaultSceneRoot`)) (+ (* (`self.GetVelocity` _enenmy_target) 0.2) (`self.K2_GetActorLocation` _enenmy_target))) false false))
    (:`else`)))

(fn `UserConstructionScript`)