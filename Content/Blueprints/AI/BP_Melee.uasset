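; BP_Melee is an AI actor with health that takes damage and is destroyed when that health runs out.
; On any damage it reports a damage event to the AI damage sense at the location of the instigator's pawn, then subtracts the damage from Health.
; While Health stays positive it prints a debug hit message, otherwise it destroys itself.
; HandleSight is an empty stub, and no melee attack logic is present.
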(event `/Game/Blueprints/AI/BPI_Percetor.HandleSight`
  (params (target :type "Actor Object Reference") (location :type "Vector Structure") (SuccessfullySensed :type Boolean)))

(event `self.ReceiveAnyDamage`
  (params (Damage :type "Float (single-precision)") (DamageType :type "DamageType Object Reference") (InstigatedBy :type "Controller Object Reference") (DamageCauser :type "Actor Object Reference"))
  (`AISense_Damage.ReportDamageEvent` self InstigatedBy Damage (`self.K2_GetActorLocation` (`Controller.K2_GetPawn` InstigatedBy)))
  (bind _output_get (set `self.Health` (- (`self.Health`) Damage))) ; sets health after damage is taken
  (if (> _output_get 0.0)
    (`KismetSystemLibrary.PrintText` (`|FormatText` "Ouch I took {amount} from {instigator}." Damage InstigatedBy))
    (else
      (`self.K2_DestroyActor`) ; kills AI
    )))

(fn `UserConstructionScript`)