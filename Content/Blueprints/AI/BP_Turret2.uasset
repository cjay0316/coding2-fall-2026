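; BP_Turret2 is an AI turret that tracks a sensed target and fires bullets at it.
; HandleSight stores the sensed actor and starts firing, or clears the target when sight is lost.
; Tick rotates the pivot to lead the target using a short velocity-based prediction.
; Attack spawns BP_Bullet at the spawn point, then re-calls itself after a rounds-per-minute delay while the target stays valid.
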(event `self.ReceiveTick`
  (params (DeltaSeconds :type "Float (single-precision)"))
  (bind _enemy_target (`self.Enemy Target`))
  (`self.Enemy Target`
    (:`then`
      (`SceneComponent.K2_SetWorldRotation` (`self.Pivot`) (`KismetMathLibrary.FindLookAtRotation` (`SceneComponent.K2_GetComponentLocation` (`self.DefaultSceneRoot`)) (+ (`self.K2_GetActorLocation` _enemy_target) (* (`self.GetVelocity` _enemy_target) 0.2))) false false))
    (:`else`)))

(event `/Game/Blueprints/AI/BPI_Percetor.HandleSight`
  (params (target :type "Actor Object Reference") (location :type "Vector Structure") (SuccessfullySensed :type Boolean))
  (if SuccessfullySensed
    (set `self.Enemy Target` target)
    (`self.Attack`)
    (else
      (set `self.Enemy Target` null) ; Clear the target
    )))

(event `Attack`
  (`self.Enemy Target`
    (:`then`
      (`|SpawnActorFromClass` "/Game/Blueprints/AI/BP_Bullet.BP_Bullet_C" (`SceneComponent.K2_GetComponentToWorld` (`self.BulletSpawn`)) "Undefined" "MultiplyWithRoot" null (`self.Initial Speed`) self)
      (`KismetSystemLibrary.Delay` (/ 60.0 (`self.Rounds per minute`)))
      (`self.Attack`))
    (:`else`)))

(fn `UserConstructionScript`)