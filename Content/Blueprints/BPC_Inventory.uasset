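; BPC_Inventory is an inventory component that stores slots as an array of item enums.
; GetSlot resolves a slot's enum to its details through GetItemDetails, which scans every DT_Items row for a matching EnumName.
; SetSlot writes one slot and SetInventory replaces the whole array, each then calling its update notification, OnSlotUpdated with the index or OnSetInventory.
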(fn `GetItemDetails`
  (params (RequestedItem :type "/Game/Blueprints/E_Item Enum" :default "NewEnumerator0"))
  (returns (ItemDetails :type "/Game/Blueprints/S_Item Structure"))
  (bind _outrownames (`DataTableFunctionLibrary.GetDataTableRowNames` "/Game/Blueprints/DataTables/DT_Items.DT_Items"))
  (for _array_element _outrownames
    (bind _returnvalue (`|GetDataTableRow` "/Game/Blueprints/DataTables/DT_Items.DT_Items" _array_element)
      (:`then`
        (if (`|EnumEquality` (`.EnumName_18_6686BD1D024ACFBF8A3E5BA7620A1117` (break `/Game/Blueprints/S_Item` _returnvalue)) RequestedItem)
          (return _returnvalue) ; Give an Item
        )))))

(fn `GetSlot`
  (params (RequestedSlot :type Integer))
  (returns (ItemDetails :type "/Game/Blueprints/S_Item Structure"))
  (bind _itemdetails (`self.GetItemDetails` (`|GetArrayItem` (`self.E Invt`) RequestedSlot)))
  (return _itemdetails))

(fn `SetInventory`
  (params (`E Invt` :type "Array of /Game/Blueprints/E_Item Enum"))
  (set `self.E Invt` `E Invt`)
  (`self.OnSetInventory`))

(fn `SetSlot`
  (params (ItemType :type "/Game/Blueprints/E_Item Enum" :default "NewEnumerator0") (Index :type Integer))
  (`KismetArrayLibrary.Array_Set` (`self.E Invt`) Index ItemType)
  (`self.OnSlotUpdated` Index))