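; BP_Shopkeeper is a shopkeeper that shows a shop menu while the first-person player character is within its sphere.
; On BeginPlay it creates W_ShopkeepMenu once, passing in its BPCInventory, and prints the first inventory item's name.
; Sphere overlap events add that same widget to the viewport when the player enters and remove it when the player leaves.
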(event `self.ReceiveBeginPlay`
  (`KismetSystemLibrary.PrintText` (`|FormatText` "First inventoory item is {item}" (`.Name_3_A3E3467BB44DB97E0033F2AFF1424D64` (break `/Game/Blueprints/S_Item` (`|GetArrayItem` (`self.Inventory`))))))
  (bind _returnvalue (`|CreateWidget` :`Class` "/Game/UI/W_ShopkeepMenu.W_ShopkeepMenu_C" :`BPC_Inventory` (`self.BPC_Inventory`))))

(event `self.Sphere.OnComponentBeginOverlap`
  (params (OverlappedComponent :type "PrimitiveComponent Object Reference") (OtherActor :type "Actor Object Reference") (OtherComp :type "PrimitiveComponent Object Reference") (OtherBodyIndex :type Integer) (bFromSweep :type Boolean) (SweepResult :type "HitResult Structure (by ref)"))
  (cast `/Game/FirstPerson/Blueprints/BP_FirstPersonCharacter` OtherActor)
  (`UserWidget.AddToViewport` (stale `self.ReceiveBeginPlay` _returnvalue) 0))

(event `self.Sphere.OnComponentEndOverlap`
  (params (OverlappedComponent :type "PrimitiveComponent Object Reference") (OtherActor :type "Actor Object Reference") (OtherComp :type "PrimitiveComponent Object Reference") (OtherBodyIndex :type Integer))
  (cast `/Game/FirstPerson/Blueprints/BP_FirstPersonCharacter` OtherActor)
  (`Widget.RemoveFromParent` (stale `self.ReceiveBeginPlay` _returnvalue)))

(fn `UserConstructionScript`)