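; Stats component that tracks health, stamina and experience, displayed through a W_PlayerStats widget created at BeginPlay.
; Each stat packs into a vector; setters treat -1 as "keep current", and stamina only initializes its bar.
; Health reaching zero fades the camera and reloads the level.
; ChangeXp attempts level changes but loops without exit, and SetXp updates the health bar instead of the experience bar.
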(event `self.ReceiveBeginPlay`
  (bind (_health_x _health_y _health_z) (`KismetMathLibrary.BreakVector` (`self.Health`)))
  (bind (_stamina_x _stamina_y _stamina_z) (`KismetMathLibrary.BreakVector` (`self.Stamina`)))
  (bind (_experience_x _experience_y _experience_z) (`KismetMathLibrary.BreakVector` (`self.Experience`)))
  (`|ExecutionSequence`
    (:`then_0`
      (bind _returnvalue (`|CreateWidget` "/Game/UI/W_PlayerStats.W_PlayerStats_C"))
      (bind _output_get (set `self.PlayerStatsWidget` _returnvalue))
      (`UserWidget.AddToViewport` _output_get 0))
    (:`then_1`
      (`self.SetHealth` _health_x _health_y _health_z)
      (`ProgressBar.SetPercent` (`/Game/UI/W_PlayerStats.StaminaBar` (`self.PlayerStatsWidget`)) _stamina_z)
      (`ProgressBar.SetPercent` (`/Game/UI/W_PlayerStats.ExperienceBar` (`self.PlayerStatsWidget`)) _experience_z))))

(event `PlayerHasDied`
  (`/Engine/EditorBlueprintResources/StandardMacros.DoOnce` false
    (:`Completed`
      (`PlayerCameraManager.StartCameraFade` :`self` (`GameplayStatics.GetPlayerCameraManager` 0) :`ToAlpha` 1.0 :`Duration` 1.0 :`bHoldWhenFinished` true)
      (`KismetSystemLibrary.Delay` 2.0)
      (bind _returnvalue (`GameplayStatics.GetCurrentLevelName` true))
      (`GameplayStatics.OpenLevel` (`KismetStringLibrary.Conv_StringToName` _returnvalue)))))

(fn `ChangeHealth`
  (params (ByAmount :type "Float (double-precision)"))
  (bind (_health_x _health_y _health_z) (`KismetMathLibrary.BreakVector` (`self.Health`)))
  (bind (_health_x_2 _health_y_2 _health_z_2) (`KismetMathLibrary.BreakVector` (`self.Health`)))
  (bind _returnvalue (+ _health_z ByAmount))
  (set `self.Health` (`KismetMathLibrary.MakeVector` _health_x _health_y _returnvalue))
  (`ProgressBar.SetPercent` (`/Game/UI/W_PlayerStats.HealthBar` (`self.PlayerStatsWidget`)) (/ _health_z_2 (- _health_y_2 _health_x_2)))
  (if (<= _returnvalue 0.0)
    (`KismetSystemLibrary.PrintText` "The player has died")
    (`self.PlayerHasDied`)))

(fn `ChangeXp`
  (params (XpAmount :type "Float (double-precision)"))
  (bind (_experience_x _experience_y _experience_z) (`KismetMathLibrary.BreakVector` (`self.Experience`)))
  (bind (_experience_x_2 _experience_y_2 _experience_z_2) (`KismetMathLibrary.BreakVector` (`self.Experience`)))
  (bind (_experience_x_3 _experience_y_3 _experience_z_3) (`KismetMathLibrary.BreakVector` (`self.Experience`)))
  (bind (_experience_x_4 _experience_y_4 _experience_z_4) (`KismetMathLibrary.BreakVector` (`self.Experience`)))
  (bind (_experience_x_5 _experience_y_5 _experience_z_5) (`KismetMathLibrary.BreakVector` (`self.Experience`)))
  (bind (_experience_x_6 _experience_y_6 _experience_z_6) (`KismetMathLibrary.BreakVector` (`self.Experience`)))
  (bind (_experience_x_7 _experience_y_7 _experience_z_7) (`KismetMathLibrary.BreakVector` (`self.Experience`)))
  (bind (_experience_x_8 _experience_y_8 _experience_z_8) (`KismetMathLibrary.BreakVector` (`self.Experience`)))
  (set `self.Experience` (`KismetMathLibrary.MakeVector` _experience_x_2 _experience_y_2 (+ XpAmount _experience_z_2)))
  (if (>= _experience_z_3 _experience_y_3) :!label _label
    ; Adds XP
    (bind _result (`/Engine/EditorBlueprintResources/StandardMacros.IncrementFloat` _experience_x_7) ; increments current lvl
      (:`  `
        (set `self.Experience` (`KismetMathLibrary.MakeVector` _result _experience_y_7 _experience_z_7))
        (set `self.Experience` (`KismetMathLibrary.MakeVector` 0.0 0.0 (- _experience_z_8 _experience_y_8)))
        (`ProgressBar.SetPercent` (`/Game/UI/W_PlayerStats.ExperienceBar` (`self.PlayerStatsWidget`)) (/ _experience_z_6 _experience_y_6))
        (`KismetSystemLibrary.PrintText` "You leveld up!")
        (goto _label)))
    (else
      ; Loses XP
      (bind _result_2 (`/Engine/EditorBlueprintResources/StandardMacros.DecrementFloat` _experience_x_4) ; decements current lvl
        (:`  `
          (set `self.Experience` (`KismetMathLibrary.MakeVector` _result_2 _experience_y_4 _experience_z_4))
          (set `self.Experience` (`KismetMathLibrary.MakeVector` 0.0 0.0 (+ _experience_z _experience_y)))
          (`ProgressBar.SetPercent` (`/Game/UI/W_PlayerStats.ExperienceBar` (`self.PlayerStatsWidget`)) (/ _experience_z_5 _experience_y_5))
          (`KismetSystemLibrary.PrintText` "You lost a level! ")
          (goto _label))))))

(fn `SetHealth`
  (params (`Health X` :type "Float (double-precision)" :default -1.0) (`Health Y` :type "Float (double-precision)" :default -1.0) (`Health Z` :type "Float (double-precision)" :default -1.0))
  (locals (MinHealth :type "Float (double-precision)") (MaxHealth :type "Float (double-precision)") (CurrentHealth :type "Float (double-precision)"))
  (bind (_health_x _health_y _health_z) (`KismetMathLibrary.BreakVector` (`self.Health`)))
  ; Setting temp vars to healths current values
  (set `local.MinHealth` (`local.Health X`))
  (set `local.MaxHealth` (`local.Health Y`))
  (set `local.CurrentHealth` (`local.Health Z`))
  (if (!= `Health X` -1.0)
    (set `local.MinHealth` `Health X`))
  (if (!= `Health Y` -1.0)
    (set `local.MaxHealth` `Health Y`))
  (if (!= `Health Z` -1.0)
    (set `local.CurrentHealth` `Health Z`))
  (set `self.Health` (`KismetMathLibrary.MakeVector` (`local.MinHealth`) (`local.MaxHealth`) (`local.CurrentHealth`)))
  ; Update the widget
  (`ProgressBar.SetPercent` (`/Game/UI/W_PlayerStats.HealthBar` (`self.PlayerStatsWidget`)) (/ _health_z (- _health_y _health_x))))

(fn `SetXp`
  (params (`Xp X` :type "Float (double-precision)") (`Xp Y` :type "Float (double-precision)") (`Xp Z` :type "Float (double-precision)"))
  (locals (CurrentXp :type "Float (double-precision)") (CurrentLevel :type "Float (double-precision)") (XpToNextLevel :type "Float (double-precision)"))
  (bind (_experience_x _experience_y _experience_z) (`KismetMathLibrary.BreakVector` (`self.Experience`)))
  (bind (_experience_x_2 _experience_y_2 _experience_z_2) (`KismetMathLibrary.BreakVector` (`self.Experience`)))
  ; Setting temp vars to xps to current values
  (set `local.CurrentLevel` _experience_x_2)
  (set `local.XpToNextLevel` _experience_y_2)
  (set `local.CurrentXp` _experience_z_2)
  (if (!= `Xp X` -1.0)
    (set `local.CurrentLevel` `Xp X`))
  (if (!= `Xp Y` -1.0)
    (set `local.XpToNextLevel` `Xp Y`))
  (if (!= `Xp Z` -1.0)
    (set `local.CurrentXp` `Xp Z`) ; Did xp change
  )
  (set `self.Experience` (`KismetMathLibrary.MakeVector` (`local.CurrentLevel`) (`local.XpToNextLevel`) (`local.CurrentXp`)))
  ; Update the widget
  (`ProgressBar.SetPercent` (`/Game/UI/W_PlayerStats.HealthBar` (`self.PlayerStatsWidget`)) (/ _experience_z (- _experience_y _experience_x))))