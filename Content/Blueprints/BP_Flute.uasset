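; BP_Flute is a pickup item representing a flute that plays music when used.
; Pickup disables collision on its Cylinder mesh and returns the item type.
; Drop re-enables collision and physics, then launches the cylinder forward with a velocity-change impulse.
; Use prints a message and plays a 2D descending scale sound.
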(event `/Game/Blueprints/BPI_Item.Drop`
  (bind _cylinder (`self.Cylinder`))
  (`PrimitiveComponent.SetCollisionEnabled` _cylinder "QueryAndPhysics")
  (`PrimitiveComponent.SetSimulatePhysics` _cylinder true)
  (`PrimitiveComponent.AddImpulse` _cylinder (* (`SceneComponent.GetForwardVector` _cylinder) 1000.0) "None" true))

(event `/Game/Blueprints/BPI_Item.Use`
  (`KismetSystemLibrary.PrintText` "Interesting music plays")
  (`GameplayStatics.PlaySound2D` "/Engine/VREditor/Sounds/VR_shep_scale_down_04.VR_shep_scale_down_04" 1.0 1.0 0.0 null null))

(fn `Pickup`
  (params (Owner :type "/Game/Blueprints/BPC_Interact Object Reference (by ref)"))
  (returns (ItemType :type "/Game/Blueprints/E_Item Enum"))
  (`PrimitiveComponent.SetCollisionEnabled` (`self.Cylinder`) "NoCollision")
  (return (`self.ItemType`)))

(fn `UserConstructionScript`)